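; EnemyRangeBP is a ranged enemy that chases the player and fires fireballs on sight.
; When PawnSensing sees a PrimaryCharacter, it starts an AI MoveTo toward that character and attempts a shot.
; Each shot spawns a FireballProjectile at ProjectileSpawnLocation and launches it by impulse along the Cube's forward vector.
; A SpawnProjectile flag reset after a short Delay serves as the fire-rate cooldown.
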(event `self.PawnSensing.OnSeePawn`
  (params (Pawn :type "Pawn Object Reference"))
  (bind _asprimary_character (cast `/Game/ThirdPersonBP/Blueprints/PrimaryCharacter` Pawn))
  (`|ExecutionSequence`
    (:`then_0`
      (`|AIMoveTo` self (0.0 0.0 0.0) _asprimary_character))
    (:`then_1`
      (if (`self.SpawnProjectile`)
        (bind _returnvalue (`|SpawnActorFromClass` "/Game/Enemies/FireballProjectile.FireballProjectile_C" (`SceneComponent.K2_GetComponentToWorld` (`self.ProjectileSpawnLocation`)) "Undefined" "OverrideRootScale"))
        (`PrimitiveComponent.AddImpulse` (`/Game/Enemies/FireballProjectile.Sphere` _returnvalue) (* (`SceneComponent.GetForwardVector` (`self.Cube`)) 2000.0) "None" true)
        (set `self.SpawnProjectile` false)
        (`KismetSystemLibrary.Delay` 1.5)
        (set `self.SpawnProjectile` true)))))

(fn `UserConstructionScript`)