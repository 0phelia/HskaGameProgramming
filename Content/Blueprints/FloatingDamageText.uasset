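; FloatingDamageText is a short-lived actor, named as floating damage text, that drifts upward and then removes itself.
; BeginPlay destroys it after a brief delay.
; Each Tick moves the root component up by the Increment variable and nudges it along positive world Y by a small random amount.
; The movement is per frame, unscaled by delta time, and the graphs shown never set any text.
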(event `self.ReceiveBeginPlay`
  (`KismetSystemLibrary.Delay` 1.5)
  (`self.K2_DestroyActor`))

(event `self.ReceiveActorBeginOverlap`
  (params (OtherActor :type "Actor Object Reference")))

(event `self.ReceiveTick`
  (params (DeltaSeconds :type "Float (single-precision)"))
  (`SceneComponent.K2_SetWorldLocation` (`self.DefaultSceneRoot`) (`KismetMathLibrary.MakeVector` (.x (`self.K2_GetActorLocation`)) (+ (.y (`self.K2_GetActorLocation`)) (`KismetMathLibrary.RandomFloatInRange` 0.0 5.0)) (+ (.z (`self.K2_GetActorLocation`)) (`self.increment`))) false false))

(fn `UserConstructionScript`)